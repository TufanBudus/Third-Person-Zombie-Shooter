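; Health pickup actor for the zombie shooter that heals a ThirdPersonCharacter on overlap.
; When its Trigger overlaps the character, it adds HealthRewarded to Health, clamped between zero and MaxHealth, and destroys itself.
; It also plays a configurable PickupSound at its location.
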(event OnComponentBeginOverlap(Trigger)
  (params (OverlappedComponent :type Primitive%20Component%20Object%20Reference) (OtherActor :type Actor%20Object%20Reference) (OtherComp :type Primitive%20Component%20Object%20Reference) (OtherBodyIndex :type Integer) (bFromSweep :type Boolean) (SweepResult :type Hit%20Result%20Structure%20%28by%20ref%29))
  (bind _asthird_person_character (Utilities|Casting|CastToThirdPersonCharacter OtherActor))
  (CallFunction|GiveHealth _asthird_person_character)
  (CallFunction|PlayPickupSound))

(event Custom|GiveHealth
  (params (WhoToGivePointsTo :type Third%20Person%20Character%20Object%20Reference))
  (Variables|/Game/ZombieShooter/Characters/BaseCharacter/ThirdPersonCharacter.ThirdPersonCharacter_C|SetHealth WhoToGivePointsTo (Math|Float|Clamp(Float) (+ (Variables|/Game/ZombieShooter/Characters/BaseCharacter/ThirdPersonCharacter.ThirdPersonCharacter_C|GetHealth WhoToGivePointsTo) (Variables|Default|GetHealthRewarded)) 0.0 (Variables|/Game/ZombieShooter/Characters/BaseCharacter/ThirdPersonCharacter.ThirdPersonCharacter_C|GetMaxHealth WhoToGivePointsTo)))
  (Actor|DestroyActor))

(event Custom|PlayPickupSound
  ;[1 1 1] Pickup Sound. Change variable to whatever sound you want
  (Audio|PlaySoundatLocation (Variables|Default|GetPickupSound) (Transformation|GetActorLocation) "0, 0, 0" 1.0 1.0 0.0 0 0 0 0))

(fn ConstructionScript)