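; Game State for the zombie shooter that handles match-wide HUD notifications, the quad points powerup and game over screens.
; Tick copies zombie and player counters from GameplayGM for debugging.
; Powerup events loop over the supplied player controllers to set or reset point multipliers and toggle the HUD timer.
; The game over event has each GameplayPC create scoreboard and game over widgets, with GameplayGM updating the scoreboard.
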(event Custom|NotificationText
  (params (NotificationText :type Text) (PlayerController :type Player%20Controller%20Object%20Reference) (Lifetime :type Float%20%28double-precision%29))
  ;[1 1 1] Notification Text such as Max ammo, double points, etc
  (bind _asgameplay_pc (Utilities|Casting|CastToGameplayPC PlayerController))
  (Utilities|IsValid (Variables|/Game/ZombieShooter/CoreBlueprints/Gameplay/GameplayPC.GameplayPC_C|GetHUDWidgetReference _asgameplay_pc)
    (:Is%20Valid
      (Default|SetNotificationText (Variables|/Game/ZombieShooter/CoreBlueprints/Gameplay/GameplayPC.GameplayPC_C|GetHUDWidgetReference _asgameplay_pc) NotificationText Lifetime))))

(event Custom|CreateGameOverWidget
  (params (AllPlayerControllers :type Array%20of%20Player%20Controller%20Object%20References))
  ;[1 1 1] Create Game Over Widget for all player controllers as well as show the scoreboard
  (for _array_element AllPlayerControllers
    (bind _asgameplay_pc (Utilities|Casting|CastToGameplayPC _array_element))
    (Default|CreateScoreboardWidget _asgameplay_pc)
    (bind _asgameplay_gm (Utilities|Casting|CastToGameplayGM (Game|GetGameMode)))
    (Default|UpdateScoreboard _asgameplay_gm)
    (Default|CreateGameOverWidget _asgameplay_pc)))

(event Custom|SetupQuadPoints
  (params (AllPlayerControllers :type Array%20of%20Player%20Controller%20Object%20References) (TimePowerupLasts :type Integer) (PointsMultiplier :type Integer))
  ;[1 1 1] Quad Points Powerup
  (Variables|Default|SetTimePowerupLasts TimePowerupLasts)
  (for _array_element AllPlayerControllers
    (bind _asgameplay_pc (Utilities|Casting|CastToGameplayPC _array_element))
    (Variables|/Game/ZombieShooter/CoreBlueprints/Gameplay/GameplayPC.GameplayPC_C|SetPointMultiplier _asgameplay_pc PointsMultiplier)
    (Utilities|IsValid (Variables|/Game/ZombieShooter/CoreBlueprints/Gameplay/GameplayPC.GameplayPC_C|GetHUDWidgetReference _asgameplay_pc)
      (:Is%20Valid
        (Widget|SetVisibility (Variables|/Game/ZombieShooter/Widgets/HUD/PlayerHUDWidget.PlayerHUDWidget_C|GetPowerUpTimer (Variables|/Game/ZombieShooter/CoreBlueprints/Gameplay/GameplayPC.GameplayPC_C|GetHUDWidgetReference _asgameplay_pc)) "Visible")))))

(event Custom|EndQuadPoints
  (params (AllPlayerControllers :type Array%20of%20Player%20Controller%20Object%20References))
  ;[1 1 1] Quad Points Powerup
  (for _array_element AllPlayerControllers
    (bind _asgameplay_pc (Utilities|Casting|CastToGameplayPC _array_element))
    (Utilities|IsValid (Variables|/Game/ZombieShooter/CoreBlueprints/Gameplay/GameplayPC.GameplayPC_C|GetHUDWidgetReference _asgameplay_pc)
      (:Is%20Valid
        (Widget|SetVisibility (Variables|/Game/ZombieShooter/Widgets/HUD/PlayerHUDWidget.PlayerHUDWidget_C|GetPowerUpTimer (Variables|/Game/ZombieShooter/CoreBlueprints/Gameplay/GameplayPC.GameplayPC_C|GetHUDWidgetReference _asgameplay_pc)) "Collapsed"))
      (:Is%20Not%20Valid
        _))
    (Variables|/Game/ZombieShooter/CoreBlueprints/Gameplay/GameplayPC.GameplayPC_C|SetPointMultiplier _asgameplay_pc 1)))

(event EventTick
  (params (DeltaSeconds :type Float%20%28single-precision%29))
  ;[1 1 1] Used for Zombie Counter Debuging. Can Remove if you don't want zombie counter
  (bind _asgameplay_gm (Utilities|Casting|CastToGameplayGM (Game|GetGameMode)))
  (Variables|DebugVariables|SetNumZombsLeft (Variables|/Game/ZombieShooter/CoreBlueprints/Gameplay/GameplayGM.GameplayGM_C|GetZombsLeftCounter _asgameplay_gm))
  (Variables|DebugVariables|SetNumZombsAlive (Variables|/Game/ZombieShooter/CoreBlueprints/Gameplay/GameplayGM.GameplayGM_C|GetZombsAliveCounter _asgameplay_gm))
  (Variables|DebugVariables|SetNumZombsPerWave (Variables|/Game/ZombieShooter/CoreBlueprints/Gameplay/GameplayGM.GameplayGM_C|GetNumZombiesPerWave _asgameplay_gm))
  (Variables|DebugVariables|SetZombSpawnCounter (Variables|/Game/ZombieShooter/CoreBlueprints/Gameplay/GameplayGM.GameplayGM_C|GetZombsSpawnCounter _asgameplay_gm))
  (Variables|DebugVariables|SetNumberOfPlayers (Variables|/Game/ZombieShooter/CoreBlueprints/Gameplay/GameplayGM.GameplayGM_C|GetNumberOfPlayers _asgameplay_gm)))

(fn ConstructionScript)