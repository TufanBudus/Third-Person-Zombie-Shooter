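; Purchasable electric trap that players activate for points, damaging actors that enter its damage trigger.
; Use triggers show cost hints and cache affordability; StartInteraction deducts points and starts a one-second counting timer.
; IsOn's RepNotify drives particles, looping audio, damage collision and net dormancy.
; IsOn clears only after the cooldown delay, keeping effects live until then; the repeating per-actor damage logic is disconnected, leaving one hit per overlap.
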(event OnComponentBeginOverlap(UseTrigger1)
  (params (OverlappedComponent :type Primitive%20Component%20Object%20Reference) (OtherActor :type Actor%20Object%20Reference) (OtherComp :type Primitive%20Component%20Object%20Reference) (OtherBodyIndex :type Integer) (bFromSweep :type Boolean) (SweepResult :type Hit%20Result%20Structure%20%28by%20ref%29))
  ;[1 1 1] Trigger Overlap Event
  (bind _asthird_person_character (Utilities|Casting|CastToThirdPersonCharacter OtherActor))
  ;;[1 1 1] Sets this variable inside Thirdperson to True which then dispatches back the start trap message.
  (Variables|/Game/ZombieShooter/Characters/BaseCharacter/ThirdPersonCharacter.ThirdPersonCharacter_C|SetShowHintstrings? _asthird_person_character true)
  (bind _asgameplay_pc (Utilities|Casting|CastToGameplayPC (Pawn|GetController _asthird_person_character)))
  (if (Variables|Default|GetIsOn?)
    (Utilities|IsValid (Variables|/Game/ZombieShooter/CoreBlueprints/Gameplay/GameplayPC.GameplayPC_C|GetHUDWidgetReference _asgameplay_pc)
      (:Is%20Valid
        (Default|SetHintstring (Variables|/Game/ZombieShooter/CoreBlueprints/Gameplay/GameplayPC.GameplayPC_C|GetHUDWidgetReference _asgameplay_pc) "Trap Already On!")))
    (else
      (if (>= (Variables|/Game/ZombieShooter/CoreBlueprints/Gameplay/GameplayPC.GameplayPC_C|GetPoints _asgameplay_pc) (Variables|Default|GetCost))
        (Variables|Default|SetCanAfford? true)
        (else
          (Variables|Default|SetCanAfford? false)))
      (Utilities|IsValid (Variables|/Game/ZombieShooter/CoreBlueprints/Gameplay/GameplayPC.GameplayPC_C|GetHUDWidgetReference _asgameplay_pc)
        (:Is%20Valid
          (Default|SetHintstring (Variables|/Game/ZombieShooter/CoreBlueprints/Gameplay/GameplayPC.GameplayPC_C|GetHUDWidgetReference _asgameplay_pc) (Utilities|Text|ToText(String) (Utilities|String|Append (Utilities|String|ToString(Text) (Variables|Default|GetHintstring)) (Utilities|String|ToString(Integer) (Variables|Default|GetCost)) " Points"))))))))

(event OnComponentEndOverlap(UseTrigger1)
  (params (OverlappedComponent :type Primitive%20Component%20Object%20Reference) (OtherActor :type Actor%20Object%20Reference) (OtherComp :type Primitive%20Component%20Object%20Reference) (OtherBodyIndex :type Integer))
  ;[1 1 1] Trigger End Overlap
  (bind _asthird_person_character (Utilities|Casting|CastToThirdPersonCharacter OtherActor))
  (Variables|/Game/ZombieShooter/Characters/BaseCharacter/ThirdPersonCharacter.ThirdPersonCharacter_C|SetShowHintstrings? _asthird_person_character false)
  (bind _asgameplay_pc (Utilities|Casting|CastToGameplayPC (Pawn|GetController _asthird_person_character)))
  (Utilities|IsValid (Variables|/Game/ZombieShooter/CoreBlueprints/Gameplay/GameplayPC.GameplayPC_C|GetHUDWidgetReference _asgameplay_pc)
    (:Is%20Valid
      (Default|SetHintstring (Variables|/Game/ZombieShooter/CoreBlueprints/Gameplay/GameplayPC.GameplayPC_C|GetHUDWidgetReference _asgameplay_pc)))))

(event OnComponentBeginOverlap(UseTrigger)
  (params (OverlappedComponent :type Primitive%20Component%20Object%20Reference) (OtherActor :type Actor%20Object%20Reference) (OtherComp :type Primitive%20Component%20Object%20Reference) (OtherBodyIndex :type Integer) (bFromSweep :type Boolean) (SweepResult :type Hit%20Result%20Structure%20%28by%20ref%29))
  ;[1 1 1] Trigger Overlap Event
  (bind _asthird_person_character (Utilities|Casting|CastToThirdPersonCharacter OtherActor))
  ;;[1 1 1] Sets this variable inside Thirdperson to True which then dispatches back the start trap message.
  (Variables|/Game/ZombieShooter/Characters/BaseCharacter/ThirdPersonCharacter.ThirdPersonCharacter_C|SetShowHintstrings? _asthird_person_character true)
  (bind _asgameplay_pc (Utilities|Casting|CastToGameplayPC (Pawn|GetController _asthird_person_character)))
  (if (Variables|Default|GetIsOn?)
    (Utilities|IsValid (Variables|/Game/ZombieShooter/CoreBlueprints/Gameplay/GameplayPC.GameplayPC_C|GetHUDWidgetReference _asgameplay_pc)
      (:Is%20Valid
        (Default|SetHintstring (Variables|/Game/ZombieShooter/CoreBlueprints/Gameplay/GameplayPC.GameplayPC_C|GetHUDWidgetReference _asgameplay_pc) "Trap Already On!")))
    (else
      (if (>= (Variables|/Game/ZombieShooter/CoreBlueprints/Gameplay/GameplayPC.GameplayPC_C|GetPoints _asgameplay_pc) (Variables|Default|GetCost))
        (Variables|Default|SetCanAfford? true)
        (else
          (Variables|Default|SetCanAfford? false)))
      (Utilities|IsValid (Variables|/Game/ZombieShooter/CoreBlueprints/Gameplay/GameplayPC.GameplayPC_C|GetHUDWidgetReference _asgameplay_pc)
        (:Is%20Valid
          (Default|SetHintstring (Variables|/Game/ZombieShooter/CoreBlueprints/Gameplay/GameplayPC.GameplayPC_C|GetHUDWidgetReference _asgameplay_pc) (Utilities|Text|ToText(String) (Utilities|String|Append (Utilities|String|ToString(Text) (Variables|Default|GetHintstring)) (Utilities|String|ToString(Integer) (Variables|Default|GetCost)) " Points"))))))))

(event OnComponentEndOverlap(UseTrigger)
  (params (OverlappedComponent :type Primitive%20Component%20Object%20Reference) (OtherActor :type Actor%20Object%20Reference) (OtherComp :type Primitive%20Component%20Object%20Reference) (OtherBodyIndex :type Integer))
  ;[1 1 1] Trigger End Overlap
  (bind _asthird_person_character (Utilities|Casting|CastToThirdPersonCharacter OtherActor))
  (Variables|/Game/ZombieShooter/Characters/BaseCharacter/ThirdPersonCharacter.ThirdPersonCharacter_C|SetShowHintstrings? _asthird_person_character false)
  (bind _asgameplay_pc (Utilities|Casting|CastToGameplayPC (Pawn|GetController _asthird_person_character)))
  (Utilities|IsValid (Variables|/Game/ZombieShooter/CoreBlueprints/Gameplay/GameplayPC.GameplayPC_C|GetHUDWidgetReference _asgameplay_pc)
    (:Is%20Valid
      (Default|SetHintstring (Variables|/Game/ZombieShooter/CoreBlueprints/Gameplay/GameplayPC.GameplayPC_C|GetHUDWidgetReference _asgameplay_pc)))))

(event OnComponentBeginOverlap(DamageTrigger)
  (params (OverlappedComponent :type Primitive%20Component%20Object%20Reference) (OtherActor :type Actor%20Object%20Reference) (OtherComp :type Primitive%20Component%20Object%20Reference) (OtherBodyIndex :type Integer) (bFromSweep :type Boolean) (SweepResult :type Hit%20Result%20Structure%20%28by%20ref%29))
  ;[1 1 1] Damage Trigger Damage Timer That Starts and Stops When Characters Overlap
  (Game|Damage|ApplyDamage OtherActor (Variables|Default|GetDamageAmmount) 0 0))

(event OnComponentEndOverlap(DamageTrigger)
  (params (OverlappedComponent :type Primitive%20Component%20Object%20Reference) (OtherActor :type Actor%20Object%20Reference) (OtherComp :type Primitive%20Component%20Object%20Reference) (OtherBodyIndex :type Integer))
  ;[1 1 1] Damage Trigger Damage Timer That Starts and Stops When Characters Overlap
)

(event Custom|StartTrap
  (params (PersonWhoActivated :type Third%20Person%20Character%20Object%20Reference))
  ;[1 1 1] Start Trap
  (bind _asgameplay_pc (Utilities|Casting|CastToGameplayPC (Pawn|GetController PersonWhoActivated)))
  (if (>= (Variables|/Game/ZombieShooter/CoreBlueprints/Gameplay/GameplayPC.GameplayPC_C|GetPoints _asgameplay_pc) (Variables|Default|GetCost)) ; Do You Have Enough Points?
    (Default|RemovePoints _asgameplay_pc (Variables|Default|GetCost))
    (Utilities|Time|SetTimerbyFunctionName 0 "TrapActivationTimer" 1.0 true)
    (Variables|Default|SetIsOn? true)))

(event Custom|StopTrap
  ;[1 1 1] Stop Trap
  (Class|KismetSystemLibrary|PauseTimer 0 "TrapActivationTimer")
  (Variables|Default|SetCounter 0.0)
  (Utilities|FlowControl|Delay (Variables|Default|GetCoolDownTime))
  (Variables|Default|SetIsOn? false))

(event Custom|UpdateTriggerHint
  (bind _usetrigger (Variables|Default|GetUseTrigger))
  ;[1 1 1] Updates the Hintstring for the Use Trigger
  (Collision|SetCollisionEnabled _usetrigger "NoCollision")
  (Utilities|FlowControl|Delay 0.2)
  (Collision|SetCollisionEnabled _usetrigger "QueryOnly"))

(event Custom|TrapFX
  ;[1 1 1] Start Playing Trap FX
  (for _array_element (Utilities|Array|MakeArray (Variables|Default|GetParticleSystem01) (Variables|Default|GetParticleSystem02) (Variables|Default|GetParticleSystem03) (Variables|Default|GetParticleSystem04) (Variables|Default|GetParticleSystem05))
    (Components|Activation|Activate _array_element false))
  (bind _returnvalue (Audio|SpawnSoundAttached (Variables|Default|GetTrapSound) (Variables|Default|GetNozzle01) "None" "0, 0, 0" "0, 0, 0" "KeepRelativeOffset" false 1.0 1.0 0.0 0 0))
  (Variables|Default|SetLoopingTrapAudio _returnvalue))

(event Custom|StopFX
  (bind _loopingtrapaudio (Variables|Default|GetLoopingTrapAudio))
  ;[1 1 1] Stops Playing the FX
  (for _array_element (Utilities|Array|MakeArray (Variables|Default|GetParticleSystem01) (Variables|Default|GetParticleSystem02) (Variables|Default|GetParticleSystem03) (Variables|Default|GetParticleSystem04) (Variables|Default|GetParticleSystem05))
    (Components|Activation|Deactivate _array_element))
  (Utilities|IsValid _loopingtrapaudio
    (:Is%20Valid
      (Audio|Components|Audio|FadeOut _loopingtrapaudio 1.0 0.0 "Linear" :!class /Script/Engine.AudioComponent))))

(event EventStartInteraction
  (params (CanActivate? :type Boolean) (PersonWhoActivatedIt :type Third%20Person%20Character%20Object%20Reference))
  ;[1 1 1] Start the Interaction Message Recieved From ThirdPersonCharacter Through the Interaction Interface Event
  (if CanActivate?
    (if (Variables|Default|GetCanAfford?)
      (if (Variables|Default|GetIsOn?) ; Is trap already on?
        _
        (else
          (CallFunction|StartTrap PersonWhoActivatedIt)))
      (CallFunction|UpdateTriggerHint))))

(fn ConstructionScript)

(fn TrapActivationTimer
  (if (>= (Variables|Default|GetCounter) (Variables|Default|GetTrapActiveTime))
    (CallFunction|StopTrap)
    (else
      (Variables|Default|SetCounter (+ (Variables|Default|GetCounter) 1.0)))))

(fn TriggerDamage
  (for _array_element (Variables|Default|GetActorsToDamage)
    (Game|Damage|ApplyDamage _array_element (Variables|Default|GetDamageAmmount) 0 0)))

(fn OnRepIsOn?
  (CallFunction|UpdateTriggerHint)
  (if (Variables|Default|GetIsOn?)
    (Networking|SetNetDormancy "DORM_Awake")
    (CallFunction|TrapFX)
    (Collision|SetCollisionEnabled (Variables|Default|GetDamageTrigger) "QueryOnly") ; Toggle Damage Trigger Collision
    (else
      (Networking|SetNetDormancy "DORM_DormantAll")
      (CallFunction|StopFX)
      (Collision|SetCollisionEnabled (Variables|Default|GetDamageTrigger) "NoCollision") ; Toggle Damage Trigger Collision
    )))