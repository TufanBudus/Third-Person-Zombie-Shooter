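; Developer interactable button that raises the zombie horde limit to 200 at once for stress-sized waves.
; Its trigger shows a HUD hint to overlapping players, and an allowed interaction overrides GameplayGM's concurrent and per-wave zombie counts.
; It then skips the current wave by destroying all BaseZombie actors, zeroing counters and starting intermission.
; A DoOnce and temporarily disabled trigger collision provide a short cooldown.
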(event OnComponentBeginOverlap(Trigger)
  (params (OverlappedComponent :type Primitive%20Component%20Object%20Reference) (OtherActor :type Actor%20Object%20Reference) (OtherComp :type Primitive%20Component%20Object%20Reference) (OtherBodyIndex :type Integer) (bFromSweep :type Boolean) (SweepResult :type Hit%20Result%20Structure%20%28by%20ref%29))
  ;[1 1 1] Starting Random Weapon Trigger Stuff
  (bind _asthird_person_character (Utilities|Casting|CastToThirdPersonCharacter OtherActor))
  ;;[1 1 1] Sets this variable inside Thirdperson to True which then dispatches back the start trap message.
  (Variables|/Game/ZombieShooter/Characters/BaseCharacter/ThirdPersonCharacter.ThirdPersonCharacter_C|SetShowHintstrings? _asthird_person_character true)
  (bind _asgameplay_pc (Utilities|Casting|CastToGameplayPC (Pawn|GetController _asthird_person_character)))
  (Utilities|IsValid (Variables|/Game/ZombieShooter/CoreBlueprints/Gameplay/GameplayPC.GameplayPC_C|GetHUDWidgetReference _asgameplay_pc)
    (:Is%20Valid
      (Default|SetHintstring (Variables|/Game/ZombieShooter/CoreBlueprints/Gameplay/GameplayPC.GameplayPC_C|GetHUDWidgetReference _asgameplay_pc) (Variables|Default|GetHintstring)))))

(event OnComponentEndOverlap(Trigger)
  (params (OverlappedComponent :type Primitive%20Component%20Object%20Reference) (OtherActor :type Actor%20Object%20Reference) (OtherComp :type Primitive%20Component%20Object%20Reference) (OtherBodyIndex :type Integer))
  ;[1 1 1] Starting Random Weapon Trigger Stuff
  (bind _asthird_person_character (Utilities|Casting|CastToThirdPersonCharacter OtherActor))
  (Variables|/Game/ZombieShooter/Characters/BaseCharacter/ThirdPersonCharacter.ThirdPersonCharacter_C|SetShowHintstrings? _asthird_person_character false)
  (bind _asgameplay_pc (Utilities|Casting|CastToGameplayPC (Pawn|GetController _asthird_person_character)))
  (Utilities|IsValid (Variables|/Game/ZombieShooter/CoreBlueprints/Gameplay/GameplayPC.GameplayPC_C|GetHUDWidgetReference _asgameplay_pc)
    (:Is%20Valid
      (Default|SetHintstring (Variables|/Game/ZombieShooter/CoreBlueprints/Gameplay/GameplayPC.GameplayPC_C|GetHUDWidgetReference _asgameplay_pc)))))

(event Custom|SkipWave
  (bind _asgameplay_gm (Utilities|Casting|CastToGameplayGM (Game|GetGameMode)))
  (Variables|/Game/ZombieShooter/CoreBlueprints/Gameplay/GameplayGM.GameplayGM_C|SetWaveOver? _asgameplay_gm true)
  (Utilities|FlowControl|DoOnce false :!label _label
    (:Completed
      (bind _outactors (Actor|GetAllActorsOfClass "/Game/ZombieShooter/AI_Zombie/BaseZombie.BaseZombie_C"))
      (for _array_element _outactors
        (Utilities|IsValid _array_element
          (:Is%20Valid
            (Actor|DestroyActor _array_element))))
      (Variables|/Game/ZombieShooter/CoreBlueprints/Gameplay/GameplayGM.GameplayGM_C|SetZombsLeftCounter _asgameplay_gm 0)
      (Variables|/Game/ZombieShooter/CoreBlueprints/Gameplay/GameplayGM.GameplayGM_C|SetZombsAliveCounter _asgameplay_gm 0)
      (Default|WaveIntermission _asgameplay_gm)
      (Development|PrintString "WAVE SKIPPED" true true "(R=0.148301,G=1.000000,B=0.000000,A=1.000000)")
      (Collision|SetCollisionEnabled (Variables|Default|GetTrigger) "NoCollision")
      (Collision|SetCollisionEnabled (Variables|Default|GetTrigger) "QueryOnly")
      (Collision|SetCollisionEnabled (Variables|Default|GetTrigger) "NoCollision")
      (Utilities|FlowControl|Delay 5.0)
      (Collision|SetCollisionEnabled (Variables|Default|GetTrigger) "QueryOnly")
      (goto _label Reset))))

(event Custom|ServerSetMaxZombies200
  (bind _asgameplay_gm (Utilities|Casting|CastToGameplayGM (Game|GetGameMode)))
  (Variables|/Game/ZombieShooter/CoreBlueprints/Gameplay/GameplayGM.GameplayGM_C|SetMaxNumZombsAtOnce _asgameplay_gm 200)
  (bind _output_get (Variables|/Game/ZombieShooter/CoreBlueprints/Gameplay/GameplayGM.GameplayGM_C|SetWaveOneNumOfZombies _asgameplay_gm 250))
  (Variables|/Game/ZombieShooter/CoreBlueprints/Gameplay/GameplayGM.GameplayGM_C|SetNumZombiesPerWave _asgameplay_gm _output_get)
  (CallFunction|SkipWave))

(event EventStartInteraction
  (params (CanActivate? :type Boolean) (PersonWhoActivatedIt :type Third%20Person%20Character%20Object%20Reference))
  ;[1 1 1] Starting Random Weapon Trigger Stuff
  (if CanActivate?
    (CallFunction|ServerSetMaxZombies200)))

(fn ConstructionScript)